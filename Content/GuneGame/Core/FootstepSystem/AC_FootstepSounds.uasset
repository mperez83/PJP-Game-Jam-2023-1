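; Actor component that plays footstep sounds for the Character that owns it, and destroys itself on any other owner.
; Each tick it checks that the character is moving on the ground at or above a required horizontal speed.
; A DoOnce gate reset after a delay spaces the footsteps by time rather than animation, with volume scaled by horizontal speed.
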(event `self.ReceiveBeginPlay`
  (bind _ascharacter (cast `Character` (`self.GetOwner`))
    (:`then`
      (set `self.CharacterRef` _ascharacter))
    (:`CastFailed`
      (`self.K2_DestroyComponent`))))

(event `self.ReceiveTick`
  (params (DeltaSeconds :type "Float (single-precision)"))
  (bind _charactermovement (`Character.CharacterMovement` (`self.CharacterRef`)))
  (bind _returnvalue (`KismetMathLibrary.VSizeXY` (`MovementComponent.Velocity` _charactermovement)))
  (if (and (`NavMovementComponent.IsMovingOnGround` _charactermovement) (>= _returnvalue (`self.SpeedRequired`)))
    (`/Engine/EditorBlueprintResources/StandardMacros.DoOnce` false :!label _label
      (:`Completed`
        (`GameplayStatics.PlaySoundAtLocation` "/Game/Everything_Bundle/Ultimate_SFX/Ultimate_Footstep_Sounds/Wav/CONCRETE/S_Footstep_Cue.S_Footstep_Cue" (`Actor.K2_GetActorLocation` (`self.CharacterRef`)) (struct) (`KismetMathLibrary.MapRangeClamped` _returnvalue 0.0 600.0 0.1 1.0) 1.0 0.0 null null null null)
        (`KismetSystemLibrary.Delay` (`self.DelayBetweenFootsteps`))
        (goto _label :!via `Reset`)))))