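; Game instance that owns the background music and applies the game's audio, display and graphics settings shortly after Init.
; SetMusic replaces the current track with a 2D sound that persists across level transitions, and FadeMusicOut fades it.
; ApplySettings turns stored volumes into sound class overrides on Mix_Master, then feeds GameUserSettings.
; Motion blur and bloom go through console commands, built without a space between name and value.
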(event `self.ReceiveInit`
  (`KismetSystemLibrary.Delay` 0.2)
  (`self.ApplySettings`))

(fn `ApplySettings`
  (bind _returnvalue (`GameUserSettings.GetGameUserSettings`))
  (`|ExecutionSequence`
    (:`then_0`
      (`GameplayStatics.SetSoundMixClassOverride` "/Game/GuneGame/Core/Audio/Mix_Master.Mix_Master" "/Game/GuneGame/Core/Audio/SoundClasses/SC_Master.SC_Master" (/ (`self.VolumeMaster`) 100.0) 1.0 0.0)
      (`GameplayStatics.SetSoundMixClassOverride` "/Game/GuneGame/Core/Audio/Mix_Master.Mix_Master" "/Game/GuneGame/Core/Audio/SoundClasses/SC_SFX.SC_SFX" (/ (`self.VolumeSFX`) 100.0) 1.0 0.0 false)
      (`GameplayStatics.SetSoundMixClassOverride` "/Game/GuneGame/Core/Audio/Mix_Master.Mix_Master" "/Game/GuneGame/Core/Audio/SoundClasses/SC_Music.SC_Music" (/ (`self.VolumeMusic`) 100.0) 1.0 0.0 false)
      (`GameplayStatics.SetBaseSoundMix` "/Game/GuneGame/Core/Audio/Mix_Master.Mix_Master")
      (`GameplayStatics.PushSoundMixModifier` "/Game/GuneGame/Core/Audio/Mix_Master.Mix_Master"))
    (:`then_1`
      (`GameUserSettings.SetScreenResolution` _returnvalue (`self.Resolution`))
      (`GameUserSettings.SetVSyncEnabled` _returnvalue (`self.VSync`))
      (`GameUserSettings.SetFullscreenMode` _returnvalue (`self.DisplayMode`))
      (`GameUserSettings.SetResolutionScaleValueEx` _returnvalue (`KismetMathLibrary.Conv_IntToDouble` (`self.ResolutionScale`)))
      (`GameUserSettings.SetTextureQuality` _returnvalue (`self.TextureQuality`))
      (`GameUserSettings.SetFoliageQuality` _returnvalue (`self.FoliageQuality`))
      (`GameUserSettings.SetVisualEffectQuality` _returnvalue (`self.EffectsQuality`))
      (`GameUserSettings.SetShadowQuality` _returnvalue (`self.ShadowQuality`))
      (`GameUserSettings.SetPostProcessingQuality` _returnvalue (`self.PostProcessQuality`)))
    (:`then_2`
      (`KismetSystemLibrary.ExecuteConsoleCommand` (`KismetStringLibrary.Concat_StrStr` "r.MotionBlur.Amount " (`KismetStringLibrary.Conv_DoubleToString` (`KismetMathLibrary.SelectFloat` 1.0 0.0 (`self.UseMotionBlur`)))) null)
      (`KismetSystemLibrary.ExecuteConsoleCommand` (`KismetStringLibrary.Concat_StrStr` "r.BloomQuality " (`KismetStringLibrary.Conv_IntToString` (`self.BloomIntensity`))) null))
    (:`then_3`
      (`GameUserSettings.ApplySettings` _returnvalue true))))

(fn `FadeMusicOut`
  (params (FadeOutDuration :type "Float (single-precision)"))
  (`AudioComponent.FadeOut` (`self.CurrentMusic`) FadeOutDuration 0.0 "Linear"))

(fn `SetMusic`
  (params (NewMusic :type "SoundBase Object Reference"))
  (`|ExecutionSequence`
    (:`then_0`
      (bind _currentmusic (`self.CurrentMusic`)
        (:`then`
          (`AudioComponent.Stop` _currentmusic)
          (`ActorComponent.K2_DestroyComponent` _currentmusic))
        (:`else`)))
    (:`then_1`
      (bind _returnvalue (`GameplayStatics.CreateSound2D` NewMusic 1.0 1.0 0.0 null true))
      (bind _output_get (set `self.CurrentMusic` _returnvalue))
      (`AudioComponent.Play` _output_get 0.0))))