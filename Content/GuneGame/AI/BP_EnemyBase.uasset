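; Base enemy character that carries a spawned gun, fires projectiles at target locations and randomizes its visual scale, with a rare triple-size roll.
; SCHealth damage events drive hit sounds, a timeline bulge and optional randomized knockback launches.
; Player kills award AC_Rank score, multiplied if the enemy is falling, and destruction also removes the gun.
; Tick drives a procedural sine walk bob scaled by horizontal speed.
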(event `self.ReceiveBeginPlay`
  (bind _sc_health (`self.SC_Health`))
  (bind (_randomsizeminmax_x _randomsizeminmax_y) (`KismetMathLibrary.BreakVector2D` (`self.RandomSizeMinMax`)))
  (bind _returnvalue (`KismetMathLibrary.RandomFloatInRange` _randomsizeminmax_x _randomsizeminmax_y))
  (`self.Set Held Gun` (`self.SpawnGun`))
  (add `/Game/GuneGame/Core/HealthSystem/SC_Health.OnProcessDamage` _sc_health (`|CreateDelegate` :!event `OnProcessDamage`))
  (add `/Game/GuneGame/Core/HealthSystem/SC_Health.OnDeath` _sc_health (`|CreateDelegate` :!event `OnDeath`))
  (`SceneComponent.SetRelativeScale3D` (`self.RandomSizeTarget`) (`KismetMathLibrary.Conv_DoubleToVector` (`KismetMathLibrary.SelectFloat` (* _returnvalue 3.0) _returnvalue (`KismetMathLibrary.RandomBoolWithWeight` 0.001)))))

(event `OnDeath`
  (params (Instigator :type "Controller Object Reference"))
  (bind (_returnvalue_location _returnvalue_rotation) (`KismetMathLibrary.BreakTransform` (`self.GetTransform`)))
  (bind _killscorevalue (`self.KillScoreValue`))
  (`|ExecutionSequence`
    (:`then_0`
      (if (== Instigator (`GameplayStatics.GetPlayerController` 0))
        (`/Game/GuneGame/Player/Rank/AC_Rank.AddToCurrentRankKills` (`self.GetComponentByClass` (`GameplayStatics.GetPlayerState` 0) "/Game/GuneGame/Player/Rank/AC_Rank.AC_Rank_C") 1 (`KismetMathLibrary.SelectInt` (`KismetMathLibrary.FCeil` (* _killscorevalue (`self.AirbornScoreMult`))) _killscorevalue (`|EnumEquality` (`CharacterMovementComponent.MovementMode` (`self.CharacterMovement`)) "MOVE_Falling")) (`KismetMathLibrary.MakeTransform` _returnvalue_location _returnvalue_rotation))))
    (:`then_1`
      (`GameplayStatics.PlaySoundAtLocation` "/Game/Everything_Bundle/Ultimate_SFX/Ultimate_Retro_Sounds/Wavs/Explosion_-_49/S_EnemyDeath_Cue.S_EnemyDeath_Cue" (`self.K2_GetActorLocation`) (struct) 1.0 1.0 0.0 null null null null))
    (:`then_2`
      (`self.K2_DestroyActor`))))

(event `self.ReceiveDestroyed`
  (bind _gunref (`self.GunRef`)
    (:`then`
      (`self.K2_DestroyActor` _gunref))
    (:`else`)))

(event `OnProcessDamage`
  (params (RemainingHealth :type Integer) (ActualDamageTaken :type Integer) (LocationDamageTookPlace :type "Vector Structure") (WasWeakSpotHit :type Boolean) (Direction :type "Vector Structure"))
  (bind (_knockbackheightrange_x _knockbackheightrange_y) (break `IntPoint` (`self.KnockbackHeightRange`)))
  (bind _knockbackrotdiff (`self.KnockBackRotDiff`))
  (bind (_knockbackpowerrange_x _knockbackpowerrange_y) (break `IntPoint` (`self.KnockbackPowerRange`)))
  (bind (_returnvalue_x _returnvalue_y) (`KismetMathLibrary.BreakVector` (* (`KismetMathLibrary.GreaterGreater_VectorRotator` Direction (`KismetMathLibrary.MakeRotator` 0.0 0.0 (`KismetMathLibrary.RandomFloatInRange` (* _knockbackrotdiff -1.0) _knockbackrotdiff))) (`KismetMathLibrary.RandomIntegerInRange` _knockbackpowerrange_x _knockbackpowerrange_y))))
  (`|ExecutionSequence`
    (:`then_0`
      (`/Game/GuneGame/Core/BlueprintMacroLibraries/BPML_ActorMacros.DoOnceDelay` 0.25)
      (`GameplayStatics.PlaySoundAtLocation` (select `bool` WasWeakSpotHit :`false` "/Game/Everything_Bundle/Ultimate_SFX/Real_Recorded_Guns/Wavs/Bullet_Impacts_Flybys/Body_armor_Impact/S_EnemyHit_Cue.S_EnemyHit_Cue" :`true` "/Game/Everything_Bundle/Ultimate_SFX/Bullet_Impacts_Flybys_Pro/Wavs/Body_Armor/S_EnemyWeakSpotHit_Cue.S_EnemyWeakSpotHit_Cue" :!type "SoundBase Object Reference") LocationDamageTookPlace (struct) 1.0 1.0 0.0 null null null null))
    (:`then_1`
      (bind (_direction _scalemod) (`Timeline|TL_BulgeAnim` :!via `PlayFromStart`)
        (:`Update`
          (`SceneComponent.SetRelativeScale3D` (`self.BulgeAnimTarget`) (`KismetMathLibrary.Conv_DoubleToVector` (+ (* _scalemod (`self.ScaleModMult`)) 1.0))))))
    (:`then_2`
      (if (`self.TakesKnockback`)
        (bind _charactermovement (`self.CharacterMovement`)
          (:`then`
            (`MovementComponent.StopMovementImmediately` _charactermovement)
            (`self.LaunchCharacter` (`KismetMathLibrary.MakeVector` _returnvalue_x _returnvalue_y (`KismetMathLibrary.Conv_IntToDouble` (`KismetMathLibrary.RandomIntegerInRange` _knockbackheightrange_x _knockbackheightrange_y)))))
          (:`else`))))))

(event `self.ReceiveTick`
  (params (DeltaSeconds :type "Float (single-precision)"))
  (bind _return (`/Game/GuneGame/Core/BlueprintFunctionLibraries/BPFL_UtilityFunctions.SimpleUpdateSineFunction` (`self.WalkDegrees`) 720.0 360.0 0.0 1.0 10.0))
  (`SceneComponent.K2_SetRelativeLocation` (`self.WalkAnimTarget`) (`KismetMathLibrary.MakeVector` 0.0 0.0 (* (`KismetMathLibrary.Abs` _return) (`KismetMathLibrary.MapRangeClamped` (`KismetMathLibrary.VSizeXY` (`self.GetVelocity`)) 0.0 250.0 0.0 1.0))) false false))

(fn `Set Held Gun`
  (params (NewGun :type "/Game/GuneGame/Guns/BP_GunBase Class Reference"))
  (bind _delaybetweenshotsoverride (`self.DelayBetweenShotsOverride`))
  (`|ExecutionSequence`
    (:`then_0`
      (bind _gunref (`self.GunRef`)
        (:`then`
          (`self.K2_DestroyActor` _gunref))
        (:`else`)))
    (:`then_1`
      (bind _returnvalue (`|SpawnActorFromClass` NewGun (`KismetMathLibrary.MakeTransform` (0.0 0.0 0.0)) "Undefined" "MultiplyWithRoot" null self))
      (bind _output_get (set `self.GunRef` _returnvalue))
      (`self.K2_AttachToComponent` _output_get (`self.GunHolder`) "None" "SnapToTarget" "SnapToTarget" "KeepRelative" true)
      (set `/Game/GuneGame/Guns/BP_GunBase.ShootVolumeMult` 0.4 _output_get)
      (set `/Game/GuneGame/Guns/BP_GunBase.2DShootSound` false _output_get)
      (if (!= _delaybetweenshotsoverride -1.0)
        (set `/Game/GuneGame/Guns/BP_GunBase.DelayBetweenShots` _delaybetweenshotsoverride _output_get)))))

(fn `Shoot at Location`
  (params (TargetLocation :type "Vector Structure"))
  (bind _gunref (`self.GunRef`)
    (:`then`
      (bind _returnvalue_location (`KismetMathLibrary.BreakTransform` (`SceneComponent.K2_GetComponentToWorld` (`/Game/GuneGame/Guns/BP_GunBase.TracerStartLoc` _gunref))))
      (`/Game/GuneGame/Guns/BP_GunBase.FireProjectileBullet` _gunref (`KismetMathLibrary.MakeTransform` _returnvalue_location (`KismetMathLibrary.FindLookAtRotation` _returnvalue_location TargetLocation)) (`self.ProjectileSpeedOverride`)))
    (:`else`)))

(fn `UpdateWalkSpeed`
  (params (NewWalkSpeed :type "Float (double-precision)"))
  (set `CharacterMovementComponent.MaxWalkSpeed` NewWalkSpeed (`self.CharacterMovement`)))

(fn `UserConstructionScript`)