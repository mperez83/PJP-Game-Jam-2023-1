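; BP_S is an enemy character Blueprint that spawns holding a gun and counts toward the player's rank when destroyed.
; On BeginPlay it sets its held gun and binds events to the damage and death callbacks of its SCHealth component.
; Death plays a sound at its location and destroys the actor.
; The Destroyed event adds a kill to the AC_Rank component on player 0's PlayerState, whatever the cause of destruction.
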(event `self.ReceiveBeginPlay`
  (bind _sc_health (`self.SC_Health`))
  (`self.Set Held Gun` (`self.SpawnGun`))
  (add `/Game/GuneGame/Core/HealthSystem/SC_Health.OnProcessDamage` _sc_health (`|CreateDelegate` :!event `OnProcessDamage`))
  (add `/Game/GuneGame/Core/HealthSystem/SC_Health.OnDeath` _sc_health (`|CreateDelegate` :!event `OnDeath`)))

(event `self.OnDeath`
  (params (Instigator :type "Controller Object Reference"))
  (`|ExecutionSequence`
    (:`then_0`
      (`GameplayStatics.PlaySoundAtLocation` "/Game/Everything_Bundle/Ultimate_SFX/Ultimate_Retro_Sounds/Wavs/Explosion_-_49/S_EnemyDeath_Cue.S_EnemyDeath_Cue" (`self.K2_GetActorLocation`) (struct) 1.0 1.0 0.0 null null null null))
    (:`then_1`
      (`self.K2_DestroyActor`))))

(event `self.ReceiveDestroyed`
  (`parent.ReceiveDestroyed`)
  (`/Game/GuneGame/Player/Rank/AC_Rank.AddToCurrentRankKills` (`self.GetComponentByClass` (`GameplayStatics.GetPlayerState` 0) "/Game/GuneGame/Player/Rank/AC_Rank.AC_Rank_C") 1))

(fn `UserConstructionScript`
  (`parent.UserConstructionScript`))