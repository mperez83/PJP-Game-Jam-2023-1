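; BP_C is an enemy AI character Blueprint with a sideways dive built on LaunchCharacter.
; Being launched stops its AI brain logic, and landing restarts it.
; StartDive launches it to its left with some lift; both branches of its random coin flip are identical.
; The only StartDive call in this graph is unreachable, and the damage event is empty.
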(event `OnProcessDamage_1`
  (params (RemainingHealth :type Integer) (LocationDamageTookPlace :type "Vector Structure") (WasWeakSpotHit :type Boolean)))

(event `self.OnLaunched`
  (params (LaunchVelocity :type "Vector Structure") (bXYOverride :type Boolean) (bZOverride :type Boolean))
  (`BrainComponent.StopLogic` (`AIController.BrainComponent` (`AIBlueprintHelperLibrary.GetAIController` self)) ""))

(event `self.OnLanded`
  (params (Hit :type "HitResult Structure (by ref)"))
  (`BrainComponent.RestartLogic` (`AIController.BrainComponent` (`AIBlueprintHelperLibrary.GetAIController` self))))

(event `StartDive`
  (bind (_returnvalue_x _returnvalue_y) (`KismetMathLibrary.BreakVector` (* (`self.GetActorRightVector`) (1000.0 1000.0 0.0))))
  (bind (_returnvalue_x_2 _returnvalue_y_2) (`KismetMathLibrary.BreakVector` (* (`KismetMathLibrary.MakeVector` _returnvalue_x _returnvalue_y) (-1.0 -1.0 0.0))))
  (if (`KismetMathLibrary.RandomBoolWithWeight` 0.5)
    (`self.LaunchCharacter` (`KismetMathLibrary.MakeVector` _returnvalue_x_2 _returnvalue_y_2 300.0))
    (else
      (`self.LaunchCharacter` (`KismetMathLibrary.MakeVector` _returnvalue_x_2 _returnvalue_y_2 300.0)))))

(fn `UserConstructionScript`
  (`parent.UserConstructionScript`))