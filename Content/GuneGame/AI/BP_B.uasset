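; BP_B is an AI Character that periodically leaps toward the player.
; On Tick, a one-second DoOnceDelay gate throttles a 50 percent random roll, which continues only while the character is moving on the ground.
; A successful check computes a ballistic velocity to the first player pawn's location at a fixed launch angle and applies it with LaunchCharacter, overriding current velocity.
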(event `self.ReceiveTick`
  (params (DeltaSeconds :type "Float (single-precision)"))
  (`/Game/GuneGame/Core/BlueprintMacroLibraries/BPML_ActorMacros.DoOnceDelay` 1.0)
  (if (`KismetMathLibrary.RandomBoolWithWeight` 0.5)
    (if (`NavMovementComponent.IsMovingOnGround` (`self.CharacterMovement`))
      (`self.LaunchCharacter` (`/Game/GuneGame/Core/BlueprintFunctionLibraries/BPFL_UtilityFunctions.CalculateLaunchVelocityToTarget` (`self.K2_GetActorLocation`) (`self.K2_GetActorLocation` (`GameplayStatics.GetPlayerPawn` 0)) 30.0) true true))))

(fn `UserConstructionScript`
  (`parent.UserConstructionScript`))