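; Actor component that keeps spawning enemies at BP_EnemySpawnPoint actors in the level, up to a maximum count.
; Below the cap, Tick runs down a timer whose speed and reset value both lerp with how full the cap is.
; Each spawn tries random points for one far enough from the player, then launches the enemy with that point's randomized velocity.
; Destroyed-event bindings keep the live count current.
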(event `self.ReceiveBeginPlay`
  (bind _outactors (`GameplayStatics.GetAllActorsOfClass` "/Game/GuneGame/AI/BP_EnemySpawnPoint.BP_EnemySpawnPoint_C"))
  (set `self.EnemySpawnPoints` _outactors))

(event `self.ReceiveTick`
  (params (DeltaSeconds :type "Float (single-precision)"))
  (if (not (`self.GetIfAtEnemyCap`))
    (bind _output_get (set `self.TimeUntilNextEnemySpawn` (`KismetMathLibrary.FClamp` (- (`self.TimeUntilNextEnemySpawn`) (* DeltaSeconds (`self.GetDeltaTimeMultiplier`))) 0.0 999.0)))
    (if (<= _output_get 0.0)
      (`self.SpawnNewEnemyEvent` 5)
      (set `self.TimeUntilNextEnemySpawn` (`self.GetSpawnTime`)))))

(event `SpawnNewEnemyEvent`
  (params (NumberOfTimesToTry :type Integer :default 5) (DistanceMustBeFromPlayer :type Integer :default 500))
  (bind _tempspawnpoint (`self.TempSpawnPoint`))
  (bind (_returnvalue_location _returnvalue_rotation) (`KismetMathLibrary.BreakTransform` (`Actor.GetTransform` _tempspawnpoint)))
  (bind _initiallaunchvelocity (`/Game/GuneGame/AI/BP_EnemySpawnPoint.InitialLaunchVelocity` _tempspawnpoint))
  (bind _launchvariation (`/Game/GuneGame/AI/BP_EnemySpawnPoint.LaunchVariation` _tempspawnpoint))
  (bind (_returnvalue_x _returnvalue_y _returnvalue_z) (`KismetMathLibrary.BreakVector` (+ _initiallaunchvelocity _launchvariation)))
  (bind (_returnvalue_x_2 _returnvalue_y_2 _returnvalue_z_2) (`KismetMathLibrary.BreakVector` (- _initiallaunchvelocity _launchvariation)))
  (for _ (range (+ NumberOfTimesToTry 1))
    (bind _output_get (set `self.TempSpawnPoint` (`KismetArrayLibrary.Array_Random` (`self.EnemySpawnPoints`))))
    (if (> (`Actor.GetDistanceTo` _output_get (`GameplayStatics.GetPlayerCharacter` 0)) DistanceMustBeFromPlayer)
      (bind _returnvalue (`|SpawnActorFromClass` (`self.EnemyToSpawn`) (`KismetMathLibrary.MakeTransform` _returnvalue_location _returnvalue_rotation) "Undefined" "MultiplyWithRoot" null null))
      (`/Engine/EditorBlueprintResources/StandardMacros.IsValid` _returnvalue
        (:`Is Valid`
          (`Character.LaunchCharacter` _returnvalue (`KismetMathLibrary.MakeVector` (`KismetMathLibrary.RandomFloatInRange` _returnvalue_x_2 _returnvalue_x) (`KismetMathLibrary.RandomFloatInRange` _returnvalue_y_2 _returnvalue_y) (`KismetMathLibrary.RandomFloatInRange` _returnvalue_z_2 _returnvalue_z)) false false)
          (add `Actor.OnDestroyed` _returnvalue (delegate `OnEnemyDestroyed`))
          (`/Engine/EditorBlueprintResources/StandardMacros.IncrementInt` (`self.CurrentEnemyCount`)
            (:`  `
              (break))))
        (:`Is Not Valid`
          (break))))))

(event `OnEnemyDestroyed`
  (params (DestroyedActor :type "Actor Object Reference"))
  (`/Engine/EditorBlueprintResources/StandardMacros.DecrementInt` (`self.CurrentEnemyCount`)))

(fn `GetDeltaTimeMultiplier`
  (returns (Return :type "Float (double-precision)"))
  (bind (_deltatimemultipliers_x _deltatimemultipliers_y) (`KismetMathLibrary.BreakVector2D` (`self.DeltaTimeMultipliers`)))
  (return (`KismetMathLibrary.Lerp` _deltatimemultipliers_x _deltatimemultipliers_y (`self.GetEnemyCapAlpha`))))

(fn `GetEnemyCapAlpha`
  (returns (Return :type "Float (double-precision)"))
  (return (/ (`self.CurrentEnemyCount`) (`self.MaxEnemyCount`))))

(fn `GetIfAtEnemyCap`
  (returns (Return :type Boolean))
  (return (>= (`self.CurrentEnemyCount`) (`self.MaxEnemyCount`))))

(fn `GetSpawnTime`
  (returns (Return :type "Float (double-precision)"))
  (bind (_spawntimes_x _spawntimes_y) (`KismetMathLibrary.BreakVector2D` (`self.SpawnTimes`)))
  (return (`KismetMathLibrary.Lerp` _spawntimes_x _spawntimes_y (`self.GetEnemyCapAlpha`))))