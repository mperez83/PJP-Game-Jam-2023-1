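; Enemy AI controller that runs the BT_EnemyBase behavior tree on BeginPlay and feeds it perception of the player character.
; AI Perception updates for BP_MainPlayerCharacter store the sensed player in SeenTarget and write the TargetActor and CanSeeTarget blackboard keys.
; On losing the player it clears SeenTarget and CanSeeTarget but leaves TargetActor set, with debug prints on both transitions.
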(event `self.ReceiveBeginPlay`
  (`self.RunBehaviorTree` "/Game/GuneGame/AI/BehaviorTreeMaterials/BT_EnemyBase.BT_EnemyBase"))

(event `self.AIPerception.OnTargetPerceptionUpdated`
  (params (Actor :type "Actor Object Reference") (Stimulus :type "AIStimulus Structure"))
  (bind _asbp_main_player_character (cast `/Game/GuneGame/Player/BP_MainPlayerCharacter` Actor))
  (if Stimulus_bSuccessfullySensed
    (`KismetSystemLibrary.PrintString` "SEE")
    (bind _output_get (set `self.SeenTarget` _asbp_main_player_character))
    (`BlackboardComponent.SetValueAsObject` (`AIBlueprintHelperLibrary.GetBlackboard` null) "TargetActor" _output_get)
    (`BlackboardComponent.SetValueAsBool` (`AIBlueprintHelperLibrary.GetBlackboard` null) "CanSeeTarget" true)
    (else
      (`KismetSystemLibrary.PrintString` "NOT")
      (set `self.SeenTarget` null)
      (`BlackboardComponent.SetValueAsBool` (`AIBlueprintHelperLibrary.GetBlackboard` null) "CanSeeTarget" false))))

(fn `UserConstructionScript`)