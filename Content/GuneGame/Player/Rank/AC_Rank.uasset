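; Component that drives gun-game rank progression, turning kills into rank-ups with widget, sound and particle feedback.
; Each rank resets the kill count, swaps the player's gun and changes the enemy type fed to the game state's spawn handler.
; The final rank clears enemies, disables spawner tick and spawns BP_S as the boss.
; Ranking past it fades music, eases into slow motion through a per-tick loop, then shows the win screen.
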(event `Initialize`
  (`|ExecutionSequence`
    (:`then_0`
      (bind _foundwidgets (`WidgetBlueprintLibrary.GetAllWidgetsOfClass` "/Game/GuneGame/Player/Rank/W_RankScore.W_RankScore_C"))
      (set `self.W_RankScoreRef` (`|GetArrayItem` _foundwidgets)))
    (:`then_1`
      (set `self.ScoreACRef` (`Actor.GetComponentByClass` (`self.GetOwner`) "/Game/GuneGame/Player/Score/AC_Score.AC_Score_C")))
    (:`then_2`
      (set `self.EnemySpawnHandlerACRef` (`Actor.GetComponentByClass` (`GameplayStatics.GetGameState`) "/Game/GuneGame/AI/AC_EnemySpawnHandler.AC_EnemySpawnHandler_C")))
    (:`then_3`
      (`self.SetNewRank` 0))))

(event `WinEvent`
  (`/Engine/EditorBlueprintResources/StandardMacros.DoOnce` false
    (:`Completed`
      (`|ExecutionSequence`
        (:`then_0`
          (`/Game/GuneGame/Core/BP_MainGameInstance.FadeMusicOut` (cast `/Game/GuneGame/Core/BP_MainGameInstance` (`GameplayStatics.GetGameInstance`) :!pure true) 4.5))
        (:`then_1`
          (bind _output_get (set `self.TimeDilation` (`KismetMathLibrary.FInterpTo` (`self.TimeDilation`) 0.25 (`GameplayStatics.GetWorldDeltaSeconds`) 10.0) :!label _label))
          (`GameplayStatics.SetGlobalTimeDilation` _output_get)
          (if (<= (`self.TimeDilation`) 0.25)
            (bind _returnvalue (`|CreateWidget` "/Game/GuneGame/Core/W_WinScreen.W_WinScreen_C"))
            (`UserWidget.AddToViewport` _returnvalue 0)
            (else
              (`KismetSystemLibrary.DelayUntilNextTick`)
              (goto _label))))))))

(fn `AddToCurrentRankKills`
  (params (AmountToAdd :type Integer :default 1))
  (`self.SetCurrentRankKills` (+ AmountToAdd (`self.CurrentRankKills`)))
  (`/Game/GuneGame/Player/Score/AC_Score.GotKill` (`self.ScoreACRef`)))

(fn `GetCurrentRank`
  (returns (Return :type "/Game/GuneGame/Player/Rank/SRank Structure"))
  (return (`|GetArrayItem` (`self.Ranks`) (`self.CurrentRankIndex`))))

(fn `RankUp`
  (bind _w_rankscoreref (`self.W_RankScoreRef`))
  (`self.SetNewRank` (+ (`self.CurrentRankIndex`) 1))
  (`UserWidget.PlayAnimation` _w_rankscoreref (`/Game/GuneGame/Player/Rank/W_RankScore.RankUp` _w_rankscoreref) 0.0 1 "Forward" 1.0 false)
  (`UserWidget.PlayAnimation` _w_rankscoreref (`/Game/GuneGame/Player/Rank/W_RankScore.RankTextBulge` _w_rankscoreref) 0.0 1 "Forward" 1.0 false)
  (`GameplayStatics.PlaySound2D` "/Game/Everything_Bundle/Ultimate_SFX/UI_Item_Sounds_HD_Remake/Wavs/S_RankUp_01_Cue.S_RankUp_01_Cue" 1.0 1.0 0.0 null null))

(fn `SetCurrentRankKills`
  (params (NewCurrentRankKills :type Integer))
  (bind _output_get (set `self.CurrentRankKills` NewCurrentRankKills))
  (if (>= _output_get (`.KillsRequiredToRankUp_17_7D748C7E435C4FEC335EBF889B1070FF` (break `/Game/GuneGame/Player/Rank/SRank` (`self.GetCurrentRank`))))
    (`self.RankUp`)
    (`ProgressBar.SetPercent` (`/Game/GuneGame/Player/Rank/W_RankScore.PBR_RankBar` (`self.W_RankScoreRef`)) 1.0)
    (else
      (`self.UpdateRankBarFill`))))

(fn `SetNewRank`
  (params (NewRankIndex :type Integer))
  (bind _output_get (set `self.CurrentRankIndex` NewRankIndex))
  (if (> _output_get (`KismetArrayLibrary.Array_LastIndex` (`self.Ranks`)))
    (`self.WinEvent`)
    (else
      (`|ExecutionSequence`
        (:`then_0`
          (`self.SetCurrentRankKills` 0))
        (:`then_1`
          (if (== (`self.CurrentRankIndex`) (`KismetArrayLibrary.Array_LastIndex` (`self.Ranks`)))
            (`|ExecutionSequence`
              (:`then_0`
                (bind _outactors (`GameplayStatics.GetAllActorsOfClass` "/Game/GuneGame/AI/BP_EnemyBase.BP_EnemyBase_C"))
                (for _array_element _outactors
                  (`Actor.K2_DestroyActor` _array_element)))
              (:`then_1`
                (`self.SetComponentTickEnabled` (`self.EnemySpawnHandlerACRef`) false))
              (:`then_2`
                (`|SpawnActorFromClass` "/Game/GuneGame/AI/Enemy_S/BP_S.BP_S_C" (`KismetMathLibrary.MakeTransform` (1000.0 1000.0 1000.0) (struct) (5.0 5.0 5.0)) "Undefined" "MultiplyWithRoot" null null)))
            (else
              (set `/Game/GuneGame/AI/AC_EnemySpawnHandler.EnemyToSpawn` (`|GetArrayItem` (`self.RankEnemies`) (`self.CurrentRankIndex`)) (`self.EnemySpawnHandlerACRef`)))))
        (:`then_2`
          (bind _asbp_main_player_character (cast `/Game/GuneGame/Player/BP_MainPlayerCharacter` (`GameplayStatics.GetPlayerCharacter` 0)))
          (`/Game/GuneGame/Player/BP_MainPlayerCharacter.SetHeldGun` _asbp_main_player_character (`|GetArrayItem` (`self.RankGuns`) (`self.CurrentRankIndex`)))
          (`NiagaraFunctionLibrary.SpawnSystemAtLocation` "/Game/GuneGame/Guns/NS_GunRankUp.NS_GunRankUp" (`SceneComponent.K2_GetComponentLocation` (`/Game/GuneGame/Player/BP_MainPlayerCharacter.GunHolder` _asbp_main_player_character))))
        (:`then_3`
          (`self.UpdateRankCosmetics`))))))

(fn `UpdateRankBarFill`
  (`/Game/GuneGame/Player/Rank/W_RankScore.UpdateRankFillBar` (`self.W_RankScoreRef`) (/ (`self.CurrentRankKills`) (`.KillsRequiredToRankUp_17_7D748C7E435C4FEC335EBF889B1070FF` (break `/Game/GuneGame/Player/Rank/SRank` (`self.GetCurrentRank`))))))

(fn `UpdateRankCosmetics`
  (`/Game/GuneGame/Player/Rank/W_RankScore.UpdateRankNameAndColors` (`self.W_RankScoreRef`) (`self.GetCurrentRank`)))