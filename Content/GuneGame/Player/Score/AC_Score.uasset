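; Score component that tracks the score and kill combo, displaying both through the W_RankScore widget.
; GotKill raises the combo, adds kill value times a tiered combo multiplier, spawns world points text and refills the combo timer.
; A DelayUntilNextTick loop, rather than Event Tick, drains the timer into the combo bar.
; When it empties, EndCombo resets the count with a drop sound and animation.
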(event `Initialize`
  (bind _foundwidgets (`WidgetBlueprintLibrary.GetAllWidgetsOfClass` "/Game/GuneGame/Player/Rank/W_RankScore.W_RankScore_C"))
  (bind _output_get (set `self.W_RankScoreRef` (`|GetArrayItem` _foundwidgets)))
  (`/Game/GuneGame/Player/Rank/W_RankScore.UpdateScoreText` _output_get (`self.Score`))
  (`/Game/GuneGame/Player/Rank/W_RankScore.UpdateComboText` _output_get (`self.ComboCount`)))

(event `GotKill`
  (params (KillScoreValue :type Integer) (PointsTextSpawnTrans :type "Transform Structure"))
  (bind _w_rankscoreref (`self.W_RankScoreRef`))
  (bind _returnvalue (* KillScoreValue (`self.GetComboMult`)))
  (bind _result (`/Engine/EditorBlueprintResources/StandardMacros.IncrementInt` (`self.ComboCount`))
    (:`  `
      (`/Game/GuneGame/Player/Rank/W_RankScore.UpdateComboText` (`self.W_RankScoreRef`) _result)
      (`|ExecutionSequence`
        (:`then_0`
          (if (== (`self.ComboCount`) 1)
            (`UserWidget.StopAnimation` _w_rankscoreref (`/Game/GuneGame/Player/Rank/W_RankScore.ComboDrop` _w_rankscoreref))
            (`UserWidget.PlayAnimation` _w_rankscoreref (`/Game/GuneGame/Player/Rank/W_RankScore.ComboAppear` _w_rankscoreref) 0.0 1 "Forward" 1.0 false)))
        (:`then_1`
          (`self.AddToScore` _returnvalue)
          (`|SpawnActorFromClass` "/Game/GuneGame/AI/BP_WorldPointsText.BP_WorldPointsText_C" PointsTextSpawnTrans "Undefined" "MultiplyWithRoot" null _returnvalue null)
          (bind _output_get (set `self.ComboLifeLeft` (`self.ComboMaxDuration`)))
          (if (> _output_get 0.0) :!label _label
            (bind _output_get_2 (set `self.ComboLifeLeft` (`KismetMathLibrary.FClamp` (- (`self.ComboLifeLeft`) (* (`GameplayStatics.GetWorldDeltaSeconds`) (`self.ComboDrainMult`))) 0.0 999.0)))
            (`/Game/GuneGame/Player/Rank/W_RankScore.UpdateComboBarPercent` (`self.W_RankScoreRef`) (/ _output_get_2 (`self.ComboMaxDuration`)))
            (`KismetSystemLibrary.DelayUntilNextTick`)
            (goto _label)
            (else
              (`self.EndCombo`))))))))

(fn `AddToScore`
  (params (AmountToAdd :type Integer))
  (bind _output_get (set `self.Score` (+ AmountToAdd (`self.Score`))))
  (`/Game/GuneGame/Player/Rank/W_RankScore.UpdateScoreText` (`self.W_RankScoreRef`) _output_get))

(fn `EndCombo`
  (bind _w_rankscoreref (`self.W_RankScoreRef`))
  (if (> (`self.ComboCount`) 0)
    (bind _output_get (set `self.ComboCount` 0))
    (`/Game/GuneGame/Player/Rank/W_RankScore.UpdateComboText` (`self.W_RankScoreRef`) _output_get)
    (`GameplayStatics.PlaySound2D` "/Game/Everything_Bundle/Ultimate_SFX/UI_Item_Sounds_HD_Remake/Wavs/S_ComboDrop_Cue.S_ComboDrop_Cue" 1.0 1.0 0.0 null null)
    (`UserWidget.PlayAnimation` _w_rankscoreref (`/Game/GuneGame/Player/Rank/W_RankScore.ComboDrop` _w_rankscoreref) 0.0 1 "Forward" 1.0 false)))

(fn `GetComboMult`
  (returns (Return :type "Float (double-precision)"))
  (if (and (>= (`self.ComboCount`) 0) (< (`self.ComboCount`) 3))
    (return 1.0)
    (elif (and (>= (`self.ComboCount`) 3) (< (`self.ComboCount`) 10))
      (return 1.5)
      (elif (>= (`self.ComboCount`) 10)
        (return 2.0)))))