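; Actor component that adds procedural sway to a scene component supplied through Initialize, driven by the owner's velocity.
; Each tick advances a shared sine phase that speeds up with horizontal speed.
; That sine layers constant breathing bob with speed-scaled movement offsets and pitch wobble, while vertical velocity adds opposing pitch tilt.
; Interpolation smooths the combined result, applied as relative location and pitch.
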(event `self.ReceiveTick`
  (params (DeltaSeconds :type "Float (single-precision)"))
  (`|ExecutionSequence`
    (:`then_0`
      (`self.PrepareVariables`))
    (:`then_1`
      (`self.DoBreathingLogic`))
    (:`then_2`
      (`self.DoMoveXYLogic`)
      (`self.DoMoveZLogic`))
    (:`then_3`
      (`self.ApplyFinalLocRot`))))

(fn `ApplyFinalLocRot`
  (`SceneComponent.K2_SetRelativeLocationAndRotation` (`self.SwaySC`) (`KismetMathLibrary.VInterpTo` (`SceneComponent.RelativeLocation` (`self.SwaySC`)) (`self.FinalLocationOffset`) (`GameplayStatics.GetWorldDeltaSeconds`) 6.0) (`KismetMathLibrary.MakeRotator` 0.0 (+ (`self.MoveXYPitchCur`) (`self.MoveZPitchCur`))) false false))

(fn `DoBreathingLogic`
  (set `self.FinalLocationOffset` (+ (`self.FinalLocationOffset`) (* (`KismetMathLibrary.MakeVector` 0.0 0.0 (`/Game/GuneGame/Core/BlueprintFunctionLibraries/BPFL_UtilityFunctions.SineDegreesToFloat` (`self.SwaySpeedDegrees`) 0.0 1 -0.25 0.25)) 1.0))))

(fn `DoMoveXYLogic`
  (`|ExecutionSequence`
    (:`then_0`
      (set `self.FinalLocationOffset` (+ (`self.FinalLocationOffset`) (* (`KismetMathLibrary.MakeVector` 0.0 (`/Game/GuneGame/Core/BlueprintFunctionLibraries/BPFL_UtilityFunctions.SineDegreesToFloat` (`self.SwaySpeedDegrees`) 0.0 1 -2.0 2.0) (`/Game/GuneGame/Core/BlueprintFunctionLibraries/BPFL_UtilityFunctions.SineDegreesToFloat` (`self.SwaySpeedDegrees`))) (`self.SwayScale`)))))
    (:`then_1`
      (set `self.MoveXYPitchCur` (`KismetMathLibrary.FInterpTo` (`self.MoveXYPitchCur`) (* (`/Game/GuneGame/Core/BlueprintFunctionLibraries/BPFL_UtilityFunctions.SineDegreesToFloat` (`self.SwaySpeedDegrees`) 90.0 2 -5.0 5.0) (`KismetMathLibrary.MapRangeClamped` (`self.SwayScale`) 0.0 3.0 0.0 1.0)) (`GameplayStatics.GetWorldDeltaSeconds`) 6.0)))))

(fn `DoMoveZLogic`
  (set `self.MoveZPitchCur` (`KismetMathLibrary.FInterpTo` (`self.MoveZPitchCur`) (`KismetMathLibrary.MapRangeClamped` (`self.ZVel`) -1000.0 1000.0 10.0 -10.0) (`GameplayStatics.GetWorldDeltaSeconds`) 6.0)))

(fn `Initialize`
  (params (SwaySC :type "SceneComponent Object Reference"))
  (set `self.SwaySC` SwaySC))

(fn `PrepareVariables`
  (bind _returnvalue (`Actor.GetVelocity` (`self.GetOwner`)))
  (`|ExecutionSequence`
    (:`then_0`
      (set `self.FinalLocationOffset` (0.0 0.0 0.0))
      (set `self.XYVel` (`KismetMathLibrary.VSizeXY` _returnvalue))
      (set `self.ZVel` (.z _returnvalue)))
    (:`then_1`
      (`/Game/GuneGame/Core/BlueprintFunctionLibraries/BPFL_UtilityFunctions.SimpleUpdateSineFunction` (`self.SwaySpeedDegrees`) (`KismetMathLibrary.MapRangeClamped` (`self.XYVel`) 100.0 1000.0 100.0 400.0))
      (set `self.SwayScale` (`KismetMathLibrary.FInterpTo` (`self.SwayScale`) (`KismetMathLibrary.MapRangeClamped` (`self.XYVel`) 0.0 1000.0 0.0 3.0) (`GameplayStatics.GetWorldDeltaSeconds`) 10.0)))))