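; AC_DynamicFollowThrough is an actor component that adds rotational follow-through sway to a scene component in the player's DynamicSway set.
; Initialize stores the follow-through component and a target rotation component, seeding the previous rotation from the follow-through component.
; Each tick it scales the target's frame-to-frame world rotation delta, negates it and interpolates the follow-through component's relative rotation toward it.
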(event `self.ReceiveTick`
  (params (DeltaSeconds :type "Float (single-precision)"))
  (set `self.DeltaRot` (* (`KismetMathLibrary.NormalizedDeltaRotator` (`self.PrevRot`) (`SceneComponent.K2_GetComponentRotation` (`self.TargetRotationSC`))) 3.0))
  (set `self.PrevRot` (`SceneComponent.K2_GetComponentRotation` (`self.TargetRotationSC`)))
  (`SceneComponent.K2_SetRelativeRotation` (`self.FollowThroughSC`) (`KismetMathLibrary.RInterpTo` (`SceneComponent.RelativeRotation` (`self.FollowThroughSC`)) (`KismetMathLibrary.NegateRotator` (`self.DeltaRot`)) (`GameplayStatics.GetWorldDeltaSeconds`) 5.0) false false))

(fn `Initialize`
  (params (FollowThroughSC :type "SceneComponent Object Reference") (TargetRotationSC :type "SceneComponent Object Reference"))
  (bind _output_get (set `self.FollowThroughSC` FollowThroughSC))
  (set `self.TargetRotationSC` TargetRotationSC)
  (set `self.PrevRot` (`SceneComponent.K2_GetComponentRotation` _output_get)))