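; Player character Blueprint that handles look, move and jump through Enhanced Input, plus pausing and shooting.
; BeginPlay adds the default mapping context, shows an instructions widget, and spawns a pistol attached to GunHolder as GunRef.
; Primary fire calls the gun's hitscan from the camera location, ignoring self; the trace end is the scaled camera-manager forward vector, without the start offset added.
; Pause input creates a new pause menu widget.
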(event `EnhancedInput|/Game/GuneGame/Player/Input/Actions/IA_Look`
  (params (ActionValue :type "Vector2D Structure") (ElapsedSeconds :type "Float (double-precision)") (TriggeredSeconds :type "Float (double-precision)") (InputAction :type "InputAction Object Reference" :default "/Game/GuneGame/Player/Input/Actions/IA_Look.IA_Look"))
  (:`Triggered`
    (`self.AddControllerYawInput` ActionValue_X)
    (`self.AddControllerPitchInput` ActionValue_Y)))

(event `EnhancedInput|/Game/GuneGame/Player/Input/Actions/IA_Move`
  (params (ActionValue :type "Vector2D Structure") (ElapsedSeconds :type "Float (double-precision)") (TriggeredSeconds :type "Float (double-precision)") (InputAction :type "InputAction Object Reference" :default "/Game/GuneGame/Player/Input/Actions/IA_Move.IA_Move"))
  (:`Triggered`
    (`self.AddMovementInput` (`self.GetActorRightVector`) ActionValue_X)
    (`self.AddMovementInput` (`self.GetActorForwardVector`) ActionValue_Y)))

(event `EnhancedInput|/Game/GuneGame/Player/Input/Actions/IA_Jump`
  (params (ActionValue :type Boolean) (ElapsedSeconds :type "Float (double-precision)") (TriggeredSeconds :type "Float (double-precision)") (InputAction :type "InputAction Object Reference" :default "/Game/GuneGame/Player/Input/Actions/IA_Jump.IA_Jump"))
  (:`Triggered`
    (`self.Jump`))
  (:`Completed`
    (`self.StopJumping`)))

(event `EnhancedInput|/Game/GuneGame/Player/Input/Actions/IA_Pause`
  (params (ActionValue :type Boolean) (ElapsedSeconds :type "Float (double-precision)") (TriggeredSeconds :type "Float (double-precision)") (InputAction :type "InputAction Object Reference" :default "/Game/GuneGame/Player/Input/Actions/IA_Pause.IA_Pause"))
  (:`Triggered`
    (bind _returnvalue (`|CreateWidget` "/Game/GuneGame/Player/UI/W_PauseMenu.W_PauseMenu_C"))
    (`UserWidget.AddToViewport` _returnvalue 0)))

(event `EnhancedInput|/Game/GuneGame/Player/Input/Actions/IA_Primary`
  (params (ActionValue :type Boolean) (ElapsedSeconds :type "Float (double-precision)") (TriggeredSeconds :type "Float (double-precision)") (InputAction :type "InputAction Object Reference" :default "/Game/GuneGame/Player/Input/Actions/IA_Primary.IA_Primary"))
  (bind _returnvalue (`GameplayStatics.GetPlayerCameraManager` 0))
  (:`Triggered`
    (bind _gunref (`self.GunRef`)
      (:`then`
        (`/Game/GuneGame/Guns/BP_GunBase.FireHitscanBullet` _gunref (`PlayerCameraManager.GetCameraLocation` _returnvalue) (* (`self.GetActorForwardVector` _returnvalue) 100000.0) (`|MakeArray` self :!type "Actor Object Reference")))
      (:`else`))))

(event `self.ReceiveBeginPlay`
  (bind _returnvalue (pcsubsystem `EnhancedInputLocalPlayerSubsystem` (`GameplayStatics.GetPlayerController` 0)))
  (`|ExecutionSequence`
    (:`then_0`
      (`/Engine/EditorBlueprintResources/StandardMacros.IsValid` _returnvalue
        (:`Is Valid`
          (`EnhancedInputSubsystemInterface.AddMappingContext` _returnvalue "/Game/GuneGame/Player/Input/IMC_Default.IMC_Default" 0 (struct)))))
    (:`then_1`
      (bind _returnvalue_2 (`|CreateWidget` "/Game/GuneGame/Core/W_Instructions.W_Instructions_C"))
      (`UserWidget.AddToViewport` _returnvalue_2 0))
    (:`then_2`
      (bind _returnvalue_3 (`|SpawnActorFromClass` "/Game/GuneGame/Guns/BP_Pistol.BP_Pistol_C" (`KismetMathLibrary.MakeTransform` (0.0 0.0 0.0)) "Undefined" "MultiplyWithRoot" null null))
      (bind _output_get (set `self.GunRef` _returnvalue_3))
      (`self.K2_AttachToComponent` _output_get (`self.GunHolder`) "None" "SnapToTarget" "SnapToTarget" "KeepRelative" true))))

(fn `UserConstructionScript`)