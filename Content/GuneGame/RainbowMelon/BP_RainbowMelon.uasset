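; BP_RainbowMelon is a pickup that grants the player rainbow power.
; Tick bobs MelonMesh vertically with a sine helper and spins it steadily around yaw, scaled by delta time.
; When BP_MainPlayerCharacter enters OverlapHitbox, the melon calls ActivateRainbowPower on it and destroys itself.
; The Destroyed event spawns the rainbow explosion Niagara effect and plays the activation sound at the melon's location.
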(event `self.ReceiveTick`
  (params (DeltaSeconds :type "Float (single-precision)"))
  (bind _melonmesh (`self.MelonMesh`))
  (bind _return (`/Game/GuneGame/Core/BlueprintFunctionLibraries/BPFL_UtilityFunctions.SimpleUpdateSineFunction` (`self.Degrees`) 360.0 360.0 0.0 1.0 10.0))
  (`SceneComponent.K2_SetRelativeLocation` _melonmesh (`KismetMathLibrary.MakeVector` 0.0 0.0 _return) false false)
  (`SceneComponent.K2_AddRelativeRotation` _melonmesh (`KismetMathLibrary.MakeRotator` 0.0 0.0 (* DeltaSeconds 360.0)) false false))

(event `self.OverlapHitbox.OnComponentBeginOverlap`
  (params (OverlappedComponent :type "PrimitiveComponent Object Reference") (OtherActor :type "Actor Object Reference") (OtherComp :type "PrimitiveComponent Object Reference") (OtherBodyIndex :type Integer) (bFromSweep :type Boolean) (SweepResult :type "HitResult Structure (by ref)"))
  (bind _asbp_main_player_character (cast `/Game/GuneGame/Player/BP_MainPlayerCharacter` OtherActor))
  (`/Game/GuneGame/Player/BP_MainPlayerCharacter.ActivateRainbowPower` _asbp_main_player_character)
  (`self.K2_DestroyActor`))

(event `self.ReceiveDestroyed`
  (bind (_returnvalue_location _returnvalue_rotation _returnvalue_scale) (`KismetMathLibrary.BreakTransform` (`self.GetTransform`)))
  (`NiagaraFunctionLibrary.SpawnSystemAtLocation` "/Game/GuneGame/RainbowMelon/NS_RainbowExplode.NS_RainbowExplode" _returnvalue_location _returnvalue_rotation _returnvalue_scale)
  (`GameplayStatics.PlaySoundAtLocation` "/Game/Everything_Bundle/Ultimate_SFX/UI_Item_Sounds_HD_Remake/Wavs/S_RainbowPowerActivate_Cue.S_RainbowPowerActivate_Cue" (`self.K2_GetActorLocation`) (struct) 1.0 1.0 0.0 null null null null))

(fn `UserConstructionScript`)