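; Base gun actor providing hitscan and projectile firing, each rate-limited by a shot delay, with a sound and multiple bullets per shot using random rotational spread.
; Hitscan traces apply point damage and spawn a cosmetic tracer toward the hit or trace end.
; Projectile shots spawn a configurable class with damage and optional speed override.
; Both play a recoil timeline that offsets and pitches a target component.
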(event `self.ReceiveBeginPlay`
  (`TimelineComponent.SetPlayRate` (`self.TL_FireAnim`) (`self.RecoilAnimPlayRate`)))

(event `FireHitscanBullet`
  (params (LineTraceTrans :type "Transform Structure") (Distance :type Integer) (ActorsToIgnore :type "Array of Actor Object Reference (by ref)"))
  (bind _inaccuracyoffset (`self.InaccuracyOffset`))
  (bind _inaccuracyoffset_2 (`self.InaccuracyOffset`))
  (bind _inaccuracyoffset_3 (`self.InaccuracyOffset`))
  (`/Game/GuneGame/Core/BlueprintMacroLibraries/BPML_ActorMacros.DoOnceDelay` (`self.DelayBetweenShots`))
  (`GameplayStatics.PlaySoundAtLocation` (`self.ShootSound`) (`self.K2_GetActorLocation`) (struct) (`self.ShootVolumeMult`) 1.0 0.0 null null null null)
  (for _ (range 1 (+ (`self.NumberOfBulletsToFire`) 1))
    (`|ExecutionSequence`
      (:`then_0`
        (bind _outhit (`KismetSystemLibrary.LineTraceSingle` LineTraceTrans_Location (+ LineTraceTrans_Location (* (`KismetMathLibrary.GetForwardVector` (`KismetMathLibrary.ComposeRotators` LineTraceTrans_Rotation (`KismetMathLibrary.MakeRotator` (`KismetMathLibrary.RandomFloatInRange` (* _inaccuracyoffset -1.0) _inaccuracyoffset) (`KismetMathLibrary.RandomFloatInRange` (* _inaccuracyoffset_2 -1.0) _inaccuracyoffset_2) (`KismetMathLibrary.RandomFloatInRange` (* _inaccuracyoffset_3 -1.0) _inaccuracyoffset_3)))) Distance)) "TraceTypeQuery1" false ActorsToIgnore))
        (`|ExecutionSequence`
          (:`then_0`
            (bind (_bblockinghit _binitialoverlap _time _distance _location _impactpoint _normal _impactnormal _physmat _hitactor _hitcomponent _hitbonename _bonename _hititem _elementindex _faceindex _tracestart _traceend) (`GameplayStatics.BreakHitResult` _outhit))
            (if _bblockinghit
              (`GameplayStatics.ApplyPointDamage` _hitactor (`KismetMathLibrary.Conv_IntToDouble` (`self.Damage`)) (`KismetMathLibrary.Normal` (- _traceend _tracestart)) _outhit (`Pawn.GetController` (`self.Instigator`)))))
          (:`then_1`
            (bind _tracerstartloc (`self.TracerStartLoc`)
              (:`then`
                (bind (_returnvalue_location _returnvalue_rotation) (`KismetMathLibrary.BreakTransform` (`SceneComponent.K2_GetComponentToWorld` _tracerstartloc)))
                (`|SpawnActorFromClass` "/Game/GuneGame/Guns/BP_FakeHitscanTracer.BP_FakeHitscanTracer_C" (`KismetMathLibrary.MakeTransform` _returnvalue_location _returnvalue_rotation) "Undefined" "MultiplyWithRoot" null (`KismetMathLibrary.SelectVector` _location _traceend _bblockinghit) 2.0 null))
              (:`else`)))))
      (:`then_1`
        (bind _tl_fireanim (`self.TL_FireAnim`)
          (:`then`
            (`TimelineComponent.PlayFromStart` _tl_fireanim))
          (:`else`))))))

(event `FireProjectileBullet`
  (params (SpawnTransform :type "Transform Structure") (ProjectileSpeedOverride :type "Float (double-precision)" :default 2500.0))
  (bind _inaccuracyoffset (`self.InaccuracyOffset`))
  (bind _inaccuracyoffset_2 (`self.InaccuracyOffset`))
  (bind _inaccuracyoffset_3 (`self.InaccuracyOffset`))
  (`/Game/GuneGame/Core/BlueprintMacroLibraries/BPML_ActorMacros.DoOnceDelay` (`self.DelayBetweenShots`))
  (`GameplayStatics.PlaySoundAtLocation` (`self.ShootSound`) (`self.K2_GetActorLocation`) (struct) (`self.ShootVolumeMult`) 1.0 0.0 null null null null)
  (for _ (range 1 (+ (`self.NumberOfBulletsToFire`) 1))
    (`|ExecutionSequence`
      (:`then_0`
        (`|SpawnActorFromClass` (`self.ProjectileToSpawn`) (`KismetMathLibrary.MakeTransform` (.location SpawnTransform) (`KismetMathLibrary.ComposeRotators` (.rotation SpawnTransform) (`KismetMathLibrary.MakeRotator` (`KismetMathLibrary.RandomFloatInRange` (* _inaccuracyoffset_2 -1.0) _inaccuracyoffset_2) (`KismetMathLibrary.RandomFloatInRange` (* _inaccuracyoffset_3 -1.0) _inaccuracyoffset_3) (`KismetMathLibrary.RandomFloatInRange` (* _inaccuracyoffset -1.0) _inaccuracyoffset)))) "Undefined" "MultiplyWithRoot" null (`KismetMathLibrary.SelectFloat` ProjectileSpeedOverride (`self.ProjectileBulletSpeed`) (!= ProjectileSpeedOverride -1.0)) 5.0 (`self.Damage`) (`self.Instigator`)))
      (:`then_1`
        (`TimelineComponent.PlayFromStart` (`self.TL_FireAnim`))))))

(fn `UserConstructionScript`)