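; BP_ProjectileBullet is a gun projectile actor that damages what it overlaps.
; The construction script copies InitialSpeed onto its ProjectileMovement component.
; HitboxMesh overlaps with actors other than the Instigator apply point damage along the bullet's forward vector, credited to the Instigator's controller, then destroy the bullet.
; A delay started at BeginPlay destroys it after LifeTime.
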(event `self.ReceiveBeginPlay`
  (`|ExecutionSequence`
    (:`then_1`
      (`KismetSystemLibrary.Delay` (`self.LifeTime`))
      (`self.K2_DestroyActor`))))

(event `self.HitboxMesh.OnComponentBeginOverlap`
  (params (OverlappedComponent :type "PrimitiveComponent Object Reference") (OtherActor :type "Actor Object Reference") (OtherComp :type "PrimitiveComponent Object Reference") (OtherBodyIndex :type Integer) (bFromSweep :type Boolean) (SweepResult :type "HitResult Structure (by ref)"))
  (if (!= OtherActor (`self.Instigator`))
    (`GameplayStatics.ApplyPointDamage` OtherActor (`KismetMathLibrary.Conv_IntToDouble` (`self.Damage`)) (`self.GetActorForwardVector`) (`GameplayStatics.MakeHitResult` false false 0.0 0.0 (0.0 0.0 0.0) (0.0 0.0 0.0) (0.0 0.0 1.0) (0.0 0.0 1.0) null null OtherComp) (`Pawn.GetController` (`self.Instigator`)))
    (`self.K2_DestroyActor`)))

(fn `UserConstructionScript`
  (set `ProjectileMovementComponent.InitialSpeed` (`self.InitialSpeed`) (`self.ProjectileMovement`)))