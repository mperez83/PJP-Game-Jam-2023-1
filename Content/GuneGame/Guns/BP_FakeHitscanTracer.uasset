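; BP_FakeHitscanTracer is a cosmetic bullet tracer that flies from its spawn location to EndLoc.
; BeginPlay scales the interpolation rate by inverse distance and BulletSpeedMult, giving constant travel speed regardless of range.
; Tick lerps the actor along that line without sweeping.
; On arrival, it hides the cylinder, deactivates the Niagara trail, and destroys itself after a short delay so the trail can fade.
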(event `self.ReceiveBeginPlay`
  (set `self.StartLoc` (`self.K2_GetActorLocation`))
  (set `self.DeltaMult` (* (/ 1.0 (* (`KismetMathLibrary.Vector_Distance` (`self.StartLoc`) (`self.EndLoc`)) 0.0001)) (`self.BulletSpeedMult`))))

(event `self.ReceiveTick`
  (params (DeltaSeconds :type "Float (single-precision)"))
  (bind _output_get (set `self.Alpha` (`KismetMathLibrary.FClamp` (+ (* DeltaSeconds (`self.DeltaMult`)) (`self.Alpha`)))))
  (`self.K2_SetActorLocation` (`KismetMathLibrary.VLerp` (`self.StartLoc`) (`self.EndLoc`) _output_get))
  (if (>= (`self.Alpha`) 1.0)
    (`/Engine/EditorBlueprintResources/StandardMacros.DoOnce` false
      (:`Completed`
        (`SceneComponent.SetVisibility` (`self.Cylinder`) false false)
        (`ActorComponent.Deactivate` (`self.NS_BulletTrail`))
        (`KismetSystemLibrary.Delay` 1.0)
        (`self.K2_DestroyActor`)))))

(fn `UserConstructionScript`)