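; Beam laser gun that fires rate-limited hitscan shots in response to FireHitscanBullet.
; Each bullet line-traces with random spread, applies point damage on a blocking hit, sets the Niagara beam's end point and restarts the fire animation timeline.
; A short ParticleLife countdown, reset per shot and ticked by a next-tick delay loop, switches the beam off when firing stops.
; The shot sound has its own throttle.
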(event `self.FireHitscanBullet`
  (params (LineTraceTrans :type "Transform Structure") (Distance :type Integer) (ActorsToIgnore :type "Array of Actor Object Reference (by ref)"))
  (bind _inaccuracyoffset (`self.InaccuracyOffset`))
  (bind _inaccuracyoffset_2 (`self.InaccuracyOffset`))
  (bind _inaccuracyoffset_3 (`self.InaccuracyOffset`))
  (`/Game/GuneGame/Core/BlueprintMacroLibraries/BPML_ActorMacros.DoOnceDelay` (`self.DelayBetweenShots`))
  (`|ExecutionSequence`
    (:`then_0`
      (set `self.ParticleLife` 0.1)
      (`ActorComponent.Activate` (`self.BeamFX`) false)
      (if (> (`self.ParticleLife`) 0.0) :!label _label
        (set `self.ParticleLife` (`KismetMathLibrary.FClamp` (- (`self.ParticleLife`) (`GameplayStatics.GetWorldDeltaSeconds`)) 0.0 999.0))
        (`KismetSystemLibrary.DelayUntilNextTick`)
        (goto _label)
        (else
          (`ActorComponent.Deactivate` (`self.BeamFX`)))))
    (:`then_1`
      (for _ (range 1 (+ (`self.NumberOfBulletsToFire`) 1))
        (`|ExecutionSequence`
          (:`then_0`
            (bind _outhit (`KismetSystemLibrary.LineTraceSingle` LineTraceTrans_Location (+ LineTraceTrans_Location (* (`KismetMathLibrary.GetForwardVector` (`KismetMathLibrary.ComposeRotators` LineTraceTrans_Rotation (`KismetMathLibrary.MakeRotator` (`KismetMathLibrary.RandomFloatInRange` (* _inaccuracyoffset_2 -1.0) _inaccuracyoffset_2) (`KismetMathLibrary.RandomFloatInRange` (* _inaccuracyoffset_3 -1.0) _inaccuracyoffset_3) (`KismetMathLibrary.RandomFloatInRange` (* _inaccuracyoffset -1.0) _inaccuracyoffset)))) Distance)) "TraceTypeQuery1" false ActorsToIgnore))
            (`|ExecutionSequence`
              (:`then_0`
                (bind (_bblockinghit _binitialoverlap _time _distance _location _impactpoint _normal _impactnormal _physmat _hitactor _hitcomponent _hitbonename _bonename _hititem _elementindex _faceindex _tracestart _traceend) (`GameplayStatics.BreakHitResult` _outhit))
                (if _bblockinghit
                  (`GameplayStatics.ApplyPointDamage` _hitactor (`KismetMathLibrary.Conv_IntToDouble` (`self.Damage`)) (0.0 0.0 0.0) _outhit (`Pawn.GetController` (`self.Instigator`)))))
              (:`then_1`
                (bind _beamfx (`self.BeamFX`)
                  (:`then`
                    (`NiagaraComponent.SetVariableVec3` _beamfx "endLoc" (`KismetMathLibrary.SelectVector` _location _traceend _bblockinghit)))
                  (:`else`)))))
          (:`then_1`
            (bind _tl_fireanim (`self.TL_FireAnim`)
              (:`then`
                (`TimelineComponent.PlayFromStart` _tl_fireanim))
              (:`else`))))))
    (:`then_2`
      (`/Game/GuneGame/Core/BlueprintMacroLibraries/BPML_ActorMacros.DoOnceDelay` 0.25)
      (`GameplayStatics.PlaySound2D` (`self.ShootSound`) (`self.ShootVolumeMult`) 1.0 0.0 null null))))

(fn `UserConstructionScript`
  (`parent.UserConstructionScript`))